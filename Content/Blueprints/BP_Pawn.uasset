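; BP_Pawn is a pawn that drives a battle log widget with randomly generated test entries.
; On BeginPlay it creates BP_BattleLog and adds it to the viewport.
; The SpawnEntry input builds a BattleLogEntryInfo object with random killer and killed names and a weighted-random boss flag, then passes it to the widget.
; GenerateRandomName assembles short names from random lowercase letters.
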(event EventBeginPlay
  ;[1 1 1] Create Battle Log widget
  (bind _returnvalue (UserInterface|CreateWidget "/Game/UI/BP_BattleLog.BP_BattleLog_C"))
  (UserInterface|Viewport|AddtoViewport _returnvalue 0)
  (Variables|Default|SetBattleLog _returnvalue))

(event Input|ActionEvents|InputActionSpawnEntry
  (params (Key :type Key%20Structure :default "None"))
  ;[1 1 1] Spawn new log entry
  (:Pressed
    (bind _name (CallFunction|GenerateRandomName))
    (bind _name_2 (CallFunction|GenerateRandomName))
    (bind _returnvalue (Game|ConstructObjectfromClass "/Game/Blueprints/BattleLogEntryInfo.BattleLogEntryInfo_C" self _name_2 _name (Math|Random|RandomBoolwithWeight 0.1)))
    (Default|AddEntry (Variables|Default|GetBattleLog) _returnvalue)))

(fn ConstructionScript)

(fn GenerateRandomName
  (for _index (range 1 (Math|Random|RandomIntegerinRange 5 10))
    (LocalVariables|SetTempName (Utilities|String|Append (LocalVariables|GetTempName) (.OutItem (Utilities|Array|Random (Utilities|String|GetCharacterArrayfromString "abcdefghijklmnopqrstuvwxyz"))))))
  (return (LocalVariables|GetTempName)))